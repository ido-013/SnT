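; BP_TrackingRange is a detection volume that chooses the homing target for a referenced Tracking projectile.
; Sphere overlaps maintain a list and count of BP_Player actors inside the range.
; On each entry, and on exit while players remain, the projectile's homing target becomes the first listed player's mesh.
; The target is not cleared when the last player leaves, and Tick is empty.
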(event `self.ReceiveBeginPlay`
  (set `self.HowManyPlayer` 0))

(event `self.Sphere.OnComponentBeginOverlap`
  (params (OverlappedComponent :type "PrimitiveComponent Object Reference") (OtherActor :type "Actor Object Reference") (OtherComp :type "PrimitiveComponent Object Reference") (OtherBodyIndex :type Integer) (bFromSweep :type Boolean) (SweepResult :type "HitResult Structure (by ref)"))
  (bind _asbp_player (cast `/Game/Merged/Player/BP_Player` OtherActor))
  (`KismetArrayLibrary.Array_Add` (`self.PlayerList`) _asbp_player)
  (set `self.HowManyPlayer` (+ (`self.HowManyPlayer`) 1))
  (set `ProjectileMovementComponent.HomingTargetComponent` (`Character.Mesh` (`|GetArrayItem` (`self.PlayerList`))) (`/Game/Hyunseok/BP_Tracking.ProjectileMovement` (`self.Tracking`))))

(event `self.Sphere.OnComponentEndOverlap`
  (params (OverlappedComponent :type "PrimitiveComponent Object Reference") (OtherActor :type "Actor Object Reference") (OtherComp :type "PrimitiveComponent Object Reference") (OtherBodyIndex :type Integer))
  (bind _playerlist (`self.PlayerList`))
  (bind _asbp_player (cast `/Game/Merged/Player/BP_Player` OtherActor))
  (bind _output_get (set `self.HowManyPlayer` (- (`self.HowManyPlayer`) 1)))
  (`KismetArrayLibrary.Array_RemoveItem` _playerlist _asbp_player)
  (`KismetArrayLibrary.Array_Resize` _playerlist _output_get)
  (if (> _output_get 0)
    (set `ProjectileMovementComponent.HomingTargetComponent` (`Character.Mesh` (`|GetArrayItem` (`self.PlayerList`))) (`/Game/Hyunseok/BP_Tracking.ProjectileMovement` (`self.Tracking`)))))

(fn `UserConstructionScript`)