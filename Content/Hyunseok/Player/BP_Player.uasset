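; Player pawn with Enhanced Input flight movement: look, move, up/down and a gauge-limited dash.
; Backward input only brakes forward motion, while dash swaps fly speed and acceleration as its gauge drains and refills on Tick.
; Slow overlaps rewrite fly speed around a delay without actually reducing it below basic speed.
; Stun and knockback flags gate input, but their trigger logic is disconnected; capsule hits only print the actor name.
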(event `self.ReceiveBeginPlay`
  (bind `_as플레이어_컨트롤러` (cast `PlayerController` (`self.GetController`)))
  (bind _returnvalue (pcsubsystem `EnhancedInputLocalPlayerSubsystem` `_as플레이어_컨트롤러`))
  (`/Engine/EditorBlueprintResources/StandardMacros.IsValid` _returnvalue
    (:`Is Valid`
      (`EnhancedInputSubsystemInterface.AddMappingContext` _returnvalue "/Game/Hyunseok/Player/Input/IMC_Player.IMC_Player" 0 (struct))
      (set `self.DashGauge` (`self.MaxDashGauge`)))))

(event `EnhancedInput|/Game/Hyunseok/Player/Input/Actions/IA_Look`
  (params (ActionValue :type "Vector2D Structure") (ElapsedSeconds :type "Float (double-precision)") (TriggeredSeconds :type "Float (double-precision)") (InputAction :type "InputAction Object Reference" :default "/Game/Hyunseok/Player/Input/Actions/IA_Look.IA_Look"))
  (:`Triggered`
    (if (not (`self.Stunned`))
      (bind _result (`/Engine/EditorBlueprintResources/StandardMacros.NegateFloat` ActionValue_X)
        (:`  `
          (`self.AddControllerYawInput` _result)
          (`self.AddControllerPitchInput` ActionValue_Y))))))

(event `EnhancedInput|/Game/Hyunseok/Player/Input/Actions/IA_Move`
  (params (ActionValue :type "Vector2D Structure") (ElapsedSeconds :type "Float (double-precision)") (TriggeredSeconds :type "Float (double-precision)") (InputAction :type "InputAction Object Reference" :default "/Game/Hyunseok/Player/Input/Actions/IA_Move.IA_Move"))
  (bind _returnvalue (`KismetMathLibrary.GetForwardVector` (`self.GetControlRotation`)))
  (:`Triggered`
    (if (`self.Stunned`)
      _
      (elif (not (`self.Knockbacked`))
        (`self.AddMovementInput` (`KismetMathLibrary.GetRightVector` (`self.GetControlRotation`)) ActionValue_X)
        (if (< ActionValue_Y 0.0)
          (if (> (`KismetMathLibrary.Dot_VectorVector` (`MovementComponent.Velocity` (`self.CharacterMovement`)) _returnvalue) 0.0)
            (`self.AddMovementInput` _returnvalue ActionValue_Y :!label _label))
          (else
            (goto _label)))))))

(event `EnhancedInput|/Game/Hyunseok/Player/Input/Actions/IA_UpDown`
  (params (ActionValue :type "Float (double-precision)") (ElapsedSeconds :type "Float (double-precision)") (TriggeredSeconds :type "Float (double-precision)") (InputAction :type "InputAction Object Reference" :default "/Game/Hyunseok/Player/Input/Actions/IA_UpDown.IA_UpDown"))
  (:`Triggered`
    (if (`self.Stunned`)
      _
      (elif (not (`self.Knockbacked`))
        (`self.AddMovementInput` (`KismetMathLibrary.GetUpVector` (`self.GetControlRotation`)) ActionValue)))))

(event `EnhancedInput|/Game/Hyunseok/Player/Input/Actions/IA_Dash`
  (params (ActionValue :type Boolean) (ElapsedSeconds :type "Float (double-precision)") (TriggeredSeconds :type "Float (double-precision)") (InputAction :type "InputAction Object Reference" :default "/Game/Hyunseok/Player/Input/Actions/IA_Dash.IA_Dash"))
  (bind _charactermovement (`self.CharacterMovement`))
  (bind _charactermovement_2 (`self.CharacterMovement`))
  (:`Triggered`
    (if (> (`self.DashGauge`) 0)
      (set `CharacterMovementComponent.MaxFlySpeed` (`self.DashSpeed`) _charactermovement)
      (set `CharacterMovementComponent.MaxAcceleration` (`self.DashSpeed`) _charactermovement_2)
      (set `self.IsDash` true)
      (else
        (set `CharacterMovementComponent.MaxFlySpeed` (`self.BasicSpeed`) _charactermovement :!label _label_2)
        (set `CharacterMovementComponent.MaxAcceleration` (`self.BasicSpeed`) _charactermovement_2)
        (set `self.IsDash` false))))
  (:`Completed`
    (goto _label_2)))

(event `self.ReceiveTick`
  (params (DeltaSeconds :type "Float (single-precision)"))
  (if (`self.IsDash`)
    (bind _result (`/Engine/EditorBlueprintResources/StandardMacros.DecrementInt` (`self.DashGauge`))
      (:`  `
        (set `self.DashGauge` _result)))
    (else
      (bind _result_2 (`/Engine/EditorBlueprintResources/StandardMacros.IncrementInt` (`self.DashGauge`))
        (:`  `
          (set `self.DashGauge` _result_2)))))
  (bind _output_get (set `self.DashGauge` (`KismetMathLibrary.Clamp` (`self.DashGauge`) 0 (`self.MaxDashGauge`)))))

(event `self.CapsuleComponent.OnComponentHit`
  (params (HitComponent :type "PrimitiveComponent Object Reference") (OtherActor :type "Actor Object Reference") (OtherComp :type "PrimitiveComponent Object Reference") (NormalImpulse :type "Vector Structure") (Hit :type "HitResult Structure (by ref)"))
  (`KismetSystemLibrary.PrintString` (`KismetSystemLibrary.GetDisplayName` OtherActor)))

(event `self.CapsuleComponent.OnComponentBeginOverlap`
  (params (OverlappedComponent :type "PrimitiveComponent Object Reference") (OtherActor :type "Actor Object Reference") (OtherComp :type "PrimitiveComponent Object Reference") (OtherBodyIndex :type Integer) (bFromSweep :type Boolean) (SweepResult :type "HitResult Structure (by ref)"))
  (bind _charactermovement (`self.CharacterMovement`))
  (switch `ECollisionChannel` (`PrimitiveComponent.GetCollisionObjectType` (`self.GetComponentByClass` OtherActor "/Script/Engine.PrimitiveComponent"))
    (:`ECC_GameTraceChannel2`
      (if (not (`self.Slowed`))
        (`KismetSystemLibrary.PrintString` "slow")
        (set `self.Slowed` true)
        (set `CharacterMovementComponent.MaxFlySpeed` (`self.DashSpeed`) _charactermovement)
        (set `CharacterMovementComponent.MaxFlySpeed` (`self.BasicSpeed`) _charactermovement)
        (`KismetSystemLibrary.Delay` 2.0)
        (set `self.Slowed` false)
        (`KismetSystemLibrary.PrintString` "event occurred")
        (set `CharacterMovementComponent.MaxFlySpeed` (`self.BasicSpeed`) _charactermovement)
        (set `CharacterMovementComponent.MaxFlySpeed` (`self.DashSpeed`) _charactermovement)))))

(fn `UserConstructionScript`)