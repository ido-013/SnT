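; BP_TrackManager runs a single-player timed race on a track.
; On BeginPlay it casts player 0 to BP_Player, starts a five-second countdown, then starts racing and enables the match flag.
; Tick accumulates and prints the match time while the match runs.
; A BP_Player overlapping the EndLine component ends racing, prints the record time and stops the match.
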(event `self.ReceiveBeginPlay`
  (bind _asbp_player (cast `/Game/Juhyeok/Player/BP_Player` (`GameplayStatics.GetPlayerCharacter` 0)))
  (set `self.Player` _asbp_player)
  (`self.BeginMatch`))

(event `BeginMatch`
  (`KismetSystemLibrary.PrintString` "Start Match")
  (`/Game/Juhyeok/Player/BP_Player.StartCountdown` (`self.Player`) 5.0)
  (`KismetSystemLibrary.Delay` 5.0)
  (`KismetSystemLibrary.PrintString` "Start Racing")
  (`/Game/Juhyeok/Player/BP_Player.StartRacing` (`self.Player`))
  (set `self.IsMatch` true))

(event `self.EndLine.OnComponentBeginOverlap`
  (params (OverlappedComponent :type "PrimitiveComponent Object Reference") (OtherActor :type "Actor Object Reference") (OtherComp :type "PrimitiveComponent Object Reference") (OtherBodyIndex :type Integer) (bFromSweep :type Boolean) (SweepResult :type "HitResult Structure (by ref)"))
  (if (`self.IsMatch`)
    (bind _asbp_player (cast `/Game/Juhyeok/Player/BP_Player` OtherActor))
    (`/Game/Juhyeok/Player/BP_Player.EndRacing` _asbp_player)
    (`KismetSystemLibrary.PrintString` (`KismetStringLibrary.Concat_StrStr` "Record: " (`KismetStringLibrary.TimeSecondsToString` (`self.MatchTime`))) true true (struct :`R` 1.0 :`B` 0.498859 :`A` 1.0))
    (set `self.IsMatch` false)))

(event `self.ReceiveTick`
  (params (DeltaSeconds :type "Float (single-precision)"))
  (if (`self.IsMatch`)
    (bind _output_get (set `self.MatchTime` (+ DeltaSeconds (`self.MatchTime`))))
    (`KismetSystemLibrary.PrintString` (`KismetStringLibrary.TimeSecondsToString` _output_get))))

(fn `UserConstructionScript`)