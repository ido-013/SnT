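; Flying player character with Enhanced Input movement, a gauge-based dash and a toggle between view-locked steering and free look.
; Movement follows control rotation when locked and mesh rotation otherwise, with backward input only braking forward motion.
; Tick updates the gauge, camera FOV and a towing bonus that grows with distance from a fixed point.
; That bonus adds to base or dash fly speed and acceleration, updated only while gauge remains.
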(event `EnhancedInput|/Game/Juhyeok/Player/Input/Actions/IA_Switch`
  (params (ActionValue :type Boolean) (ElapsedSeconds :type "Float (double-precision)") (TriggeredSeconds :type "Float (double-precision)") (InputAction :type "InputAction Object Reference" :default "/Game/Juhyeok/Player/Input/Actions/IA_Switch.IA_Switch"))
  (:`Started`
    (bind _output_get (set `self.FixPerspective` (not (`self.FixPerspective`))))
    (bind _output_get_2 (set `self.bUseControllerRotationPitch` _output_get))
    (bind _output_get_3 (set `self.bUseControllerRotationYaw` _output_get_2))
    (bind _output_get_4 (set `self.bUseControllerRotationRoll` _output_get_3))
    (if _output_get_4
      (`Controller.SetControlRotation` (`self.GetController`) (`self.ControlRotation`)))))

(event `self.ReceiveBeginPlay`
  (bind `_as플레이어_컨트롤러` (cast `PlayerController` (`self.GetController`)))
  (bind _returnvalue (pcsubsystem `EnhancedInputLocalPlayerSubsystem` `_as플레이어_컨트롤러`))
  (`/Engine/EditorBlueprintResources/StandardMacros.IsValid` _returnvalue
    (:`Is Valid`
      (`EnhancedInputSubsystemInterface.AddMappingContext` _returnvalue "/Game/Juhyeok/Player/Input/IMC_Player.IMC_Player" 0 (struct))
      (set `self.DashGauge` (`self.MaxDashGauge`))
      (set `self.ControlRotation` (`self.GetControlRotation`)))))

(event `EnhancedInput|/Game/Juhyeok/Player/Input/Actions/IA_Look`
  (params (ActionValue :type "Vector2D Structure") (ElapsedSeconds :type "Float (double-precision)") (TriggeredSeconds :type "Float (double-precision)") (InputAction :type "InputAction Object Reference" :default "/Game/Juhyeok/Player/Input/Actions/IA_Look.IA_Look"))
  (:`Triggered`
    (bind _result (`/Engine/EditorBlueprintResources/StandardMacros.NegateFloat` ActionValue_X)
      (:`  `
        (`self.AddControllerYawInput` _result)
        (`self.AddControllerPitchInput` ActionValue_Y)))))

(event `EnhancedInput|/Game/Juhyeok/Player/Input/Actions/IA_Move`
  (params (ActionValue :type "Vector2D Structure") (ElapsedSeconds :type "Float (double-precision)") (TriggeredSeconds :type "Float (double-precision)") (InputAction :type "InputAction Object Reference" :default "/Game/Juhyeok/Player/Input/Actions/IA_Move.IA_Move"))
  (bind _returnvalue (`KismetMathLibrary.GetForwardVector` (`self.ReferenceRotation`)))
  (:`Triggered`
    (`self.Set Reference Rotation`)
    (`self.AddMovementInput` (`KismetMathLibrary.GetRightVector` (`self.ReferenceRotation`)) ActionValue_X)
    (if (< ActionValue_Y 0.0)
      (if (> (`KismetMathLibrary.Dot_VectorVector` (`MovementComponent.Velocity` (`self.CharacterMovement`)) _returnvalue) 0.0)
        (`self.AddMovementInput` _returnvalue ActionValue_Y :!label _label))
      (else
        (goto _label)))))

(event `EnhancedInput|/Game/Juhyeok/Player/Input/Actions/IA_UpDown`
  (params (ActionValue :type "Float (double-precision)") (ElapsedSeconds :type "Float (double-precision)") (TriggeredSeconds :type "Float (double-precision)") (InputAction :type "InputAction Object Reference" :default "/Game/Juhyeok/Player/Input/Actions/IA_UpDown.IA_UpDown"))
  (:`Triggered`
    (`self.AddMovementInput` (`KismetMathLibrary.GetUpVector` (`self.GetControlRotation`)) ActionValue)))

(event `EnhancedInput|/Game/Juhyeok/Player/Input/Actions/IA_Dash`
  (params (ActionValue :type Boolean) (ElapsedSeconds :type "Float (double-precision)") (TriggeredSeconds :type "Float (double-precision)") (InputAction :type "InputAction Object Reference" :default "/Game/Juhyeok/Player/Input/Actions/IA_Dash.IA_Dash"))
  (:`Triggered`
    (set `self.IsDash` true))
  (:`Completed`
    (set `self.IsDash` false)))

(event `self.ReceiveTick`
  (params (DeltaSeconds :type "Float (single-precision)"))
  (`self.Set Dash Gauge`)
  (set `self.TowingSpeed` (`KismetMathLibrary.FClamp` (/ (`KismetMathLibrary.Vector_Distance` (`self.K2_GetActorLocation`) (0.0 0.0 500.0)) 5.0) 0.0 500.0))
  (`self.Set Speed`)
  (set `CameraComponent.FieldOfView` (`self.Get FOV`) (`self.Camera`)))

(fn `UserConstructionScript`)