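; BP_SeahorseProj is the player seahorse's projectile, which swells and slows as it travels.
; While it moves fast enough, each Tick grows the sphere's scale and damps velocity by fixed per-frame steps, independent of delta time.
; Any overlap zeroes velocity and flags it attached, halting growth without actually attaching it; overlapping a Pawn-type collider destroys it.
; A lifetime timer accumulated on Tick destroys it otherwise.
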(event `self.ReceiveActorBeginOverlap`
  (params (OtherActor :type "Actor Object Reference"))
  (set `self.OtherCollisionType` (`PrimitiveComponent.GetCollisionObjectType` (`self.GetComponentByClass` OtherActor "/Script/Engine.PrimitiveComponent")))
  (set `MovementComponent.Velocity` (0.0 0.0 0.0) (`self.ProjectileMovement`))
  (set `self.IsAttached` true)
  (switch `ECollisionChannel` (`self.OtherCollisionType`)
    (:`ECC_Pawn`
      (`self.K2_DestroyActor`))))

(event `self.ReceiveTick`
  (params (DeltaSeconds :type "Float (single-precision)"))
  (bind _output_get (set `self.DestroyTimer` (+ DeltaSeconds (`self.DestroyTimer`))))
  (if (> _output_get (`self.MaxDestroyTimer`))
    (`self.K2_DestroyActor`)
    (elif (not (`self.IsAttached`))
      (`self.Set Projectile Attr` 50.0 0.02 10.0 0.99))))

(fn `UserConstructionScript`)