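; BP_PenguinProj is a penguin projectile that deflects off what its sphere overlaps and destroys itself on overlapping a pawn.
; Sphere overlaps redirect ProjectileMovement velocity along the sweep normal while preserving speed, rather than computing a true reflection.
; Actor overlaps check the collision object type of the other actor's primitive component for Pawn.
; A Tick-accumulated timer destroys the projectile once it exceeds MaxDestroyTimer.
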(event `self.ReceiveActorBeginOverlap`
  (params (OtherActor :type "Actor Object Reference"))
  (set `self.OtherCollisionType` (`PrimitiveComponent.GetCollisionObjectType` (`self.GetComponentByClass` OtherActor "/Script/Engine.PrimitiveComponent")))
  (switch `ECollisionChannel` (`self.OtherCollisionType`)
    (:`ECC_Pawn`
      (`self.K2_DestroyActor`))))

(event `self.ReceiveTick`
  (params (DeltaSeconds :type "Float (single-precision)"))
  (bind _output_get (set `self.DestroyTimer` (+ DeltaSeconds (`self.DestroyTimer`))))
  (if (> _output_get (`self.MaxDestroyTimer`))
    (`self.K2_DestroyActor`)))

(event `self.Sphere.OnComponentBeginOverlap`
  (params (OverlappedComponent :type "PrimitiveComponent Object Reference") (OtherActor :type "Actor Object Reference") (OtherComp :type "PrimitiveComponent Object Reference") (OtherBodyIndex :type Integer) (bFromSweep :type Boolean) (SweepResult :type "HitResult Structure (by ref)"))
  (set `MovementComponent.Velocity` (* SweepResult_Normal (`KismetMathLibrary.VSize` (`MovementComponent.Velocity` (`self.ProjectileMovement`)))) (`self.ProjectileMovement`)))

(fn `UserConstructionScript`)