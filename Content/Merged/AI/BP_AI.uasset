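; BP_AI is an AI actor that follows a looping series of checkpoints on a BP_AITrack.
; On BeginPlay it finds the track in the level and sets its ProjectileMovement homing target to the first checkpoint's root component.
; UpdateIndex retargets homing to the checkpoint after the one passed in, wrapping to the first when none is valid, and prints a debug string.
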(event `self.ReceiveBeginPlay`
  (bind _returnvalue (`GameplayStatics.GetActorOfClass` "/Game/Merged/AI/BP_AITrack.BP_AITrack_C"))
  (bind _output_get (set `self.Track` _returnvalue))
  (set `ProjectileMovementComponent.HomingTargetComponent` (`Actor.RootComponent` (`|GetArrayItem` (`/Game/Merged/AI/BP_AITrack.Checkpoints` _output_get))) (`self.ProjectileMovement`)))

(event `Update Index`
  (params (Checkpoint :type "/Game/Merged/Track/BP_Checkpoint Object Reference"))
  (bind _checkpoints (`/Game/Merged/AI/BP_AITrack.Checkpoints` (`self.Track`)))
  (bind _output (`|GetArrayItem` _checkpoints (+ (`KismetArrayLibrary.Array_Find` _checkpoints Checkpoint) 1)))
  (bind `_as액터` (cast `Actor` (`KismetMathLibrary.SelectObject` _output (`|GetArrayItem` _checkpoints) (`KismetSystemLibrary.IsValid` _output))))
  (set `ProjectileMovementComponent.HomingTargetComponent` (`Actor.RootComponent` `_as액터`) (`self.ProjectileMovement`))
  (`KismetSystemLibrary.PrintString` "Hello"))

(fn `UserConstructionScript`)