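; Player controller for the game result level, handling each player's profile handoff, pawn coloring and ranking display.
; On local BeginPlay it passes the profile and arrival flag from the game instance through an RPC, then shows a load screen.
; RPC events drive the CameraSetting actor, multicast player-ID colors to Seahorse or Penguin pawns, and fill result widget rows by rank with name, color and time or "Retired".
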(event `self.ReceiveBeginPlay`
  (if (`self.IsLocalPlayerController`)
    (bind _asbp_shooter_gameinstance (cast `/Game/Merged/Framework/BP_Shooter_Gameinstance` (`GameplayStatics.GetGameInstance`)))
    (bind _output_get (set `self.Player Profile Info` (`/Game/Merged/Framework/BP_Shooter_Gameinstance.PlayerProfile_Info` _asbp_shooter_gameinstance)))
    (bind _output_get_2 (set `self.IsArrived` (`/Game/Merged/Framework/BP_Shooter_Gameinstance.IsArrived` _asbp_shooter_gameinstance)))
    (`self.RPC_GetPlayerProfile` self _output_get _output_get_2)
    (`self.RPC_ShowLoadScreen`)
    (else
      (`KismetSystemLibrary.PrintString` "Not local player controller"))))

(event `RPC_GetPlayerProfile`
  (params (`Player Profile Info` :type "/Game/Merged/SavedData/S_PlayerProfile Structure") (IsArrived :type Boolean))
  (set `self.Player Profile Info` `Player Profile Info`)
  (set `self.IsArrived` IsArrived)
  (set `self.IsPlayerProfile` true))

(event `RPC_SetDefault`
  (bind _returnvalue (`GameplayStatics.GetActorOfClass` "/Game/Merged/Maps/GameResult/CameraSetting.CameraSetting_C"))
  (`/Game/Merged/Maps/GameResult/CameraSetting.SetDefault` _returnvalue self))

(event `RPC_SetTargets`
  (bind _returnvalue (`GameplayStatics.GetActorOfClass` "/Game/Merged/Maps/GameResult/CameraSetting.CameraSetting_C"))
  (`/Game/Merged/Maps/GameResult/CameraSetting.SetTargets` _returnvalue self))

(event `RPC_ShowLoadScreen`
  (`self.UI_ShowLoadScreen` self "GameResult"))

(event `RPC_RemoveLoadScreen`
  (bind _wb_loadscreen_widget (`self.WB_LoadScreen_Widget`))
  (`/Engine/EditorBlueprintResources/StandardMacros.IsValid` _wb_loadscreen_widget
    (:`Is Valid`
      (`Widget.RemoveFromParent` _wb_loadscreen_widget))))

(event `RPC_SetPlayerActorColor`
  (params (Character :type "/Game/Merged/SavedData/E_Characters Enum" :default "NewEnumerator0") (PID :type Integer))
  (bind _returnvalue (`self.K2_GetPawn` self))
  ;[1 1 1] Player Actor Color
  (`/Engine/EditorBlueprintResources/StandardMacros.IsValid` _returnvalue
    (:`Is Valid`
      (switch `/Game/Merged/SavedData/E_Characters` Character
        (:`NewEnumerator0`
          (bind _asbp_seahorse (cast `/Game/Merged/Character/Seahorse/BP_Seahorse` _returnvalue :!label _label))
          (bind _color (`self.Get_Color` self PID))
          (`self.Multicast_SetPlayerActorColor_Seahorse` self _asbp_seahorse _color))
        (:`NewEnumerator1`
          (goto _label))
        (:`NewEnumerator2`
          (bind _asbp_penguin (cast `/Game/Merged/Character/Penguin/BP_Penguin` _returnvalue))
          (bind _color_2 (`self.Get_Color` self PID))
          (`self.Multicast_SetPlayerActorColor_Penguin` self _asbp_penguin _color_2))))))

(event `Multicast_SetPlayerActorColor_Seahorse`
  (params (`타깃` :type "/Game/Merged/Character/Seahorse/BP_Seahorse Object Reference") (Value :type "LinearColor Structure"))
  ;[1 1 1] Player Actor Color
  (`/Game/Merged/Character/Seahorse/BP_Seahorse.Set_ActorColor` `타깃` Value))

(event `Multicast_SetPlayerActorColor_Penguin`
  (params (`타깃` :type "/Game/Merged/Character/Penguin/BP_Penguin Object Reference") (Value :type "LinearColor Structure"))
  ;[1 1 1] Player Actor Color
  (`/Game/Merged/Character/Penguin/BP_Penguin.Set_ActorColor` `타깃` Value))

(event `SetGameResultInfo`
  (params (Name :type Text) (Rank :type Integer) (Record :type "Timespan Structure") (PID :type Integer) (IsArrived :type Boolean))
  (bind _output (`|GetArrayItem` (`/Game/Merged/Widgets/WB_GameResult.TB_Records` (`self.WB_GameResult_Widget`)) Rank))
  (`TextBlock.SetText` (`|GetArrayItem` (`/Game/Merged/Widgets/WB_GameResult.TB_PlayerNames` (`self.WB_GameResult_Widget`)) Rank) Name)
  (bind _color (`self.Get_Color` PID))
  (`Border.SetBrushColor` (`|GetArrayItem` (`/Game/Merged/Widgets/WB_GameResult.RankBorders` (`self.WB_GameResult_Widget`)) Rank) _color)
  (if IsArrived
    (`TextBlock.SetText` _output (`KismetTextLibrary.AsTimespan_Timespan` Record))
    (else
      (`TextBlock.SetText` _output "Retired"))))

(event `RPC_SetGameResultInfo`
  (params (Name :type Text) (Rank :type Integer) (Record :type "Timespan Structure") (PID :type Integer) (IsArrived :type Boolean))
  (`self.SetGameResultInfo` self Name Rank Record PID IsArrived))

(event `Show_GameResult`
  (bind _wb_gameresult_widget (`self.WB_GameResult_Widget`))
  (`/Engine/EditorBlueprintResources/StandardMacros.IsValid` _wb_gameresult_widget
    (:`Is Valid`
      (`/Game/Merged/Widgets/WB_GameResult.Show_GameResult` _wb_gameresult_widget))))

(event `Create_GameResultWidget`
  (`self.UI Create Game Result` self))

(fn `Get_Color`
  (params (PID :type Integer))
  (returns (Color :type "LinearColor Structure"))
  (switch `int` PID
    (:`0`
      (return (`KismetMathLibrary.MakeColor` 1.0)))
    (:`1`
      (return (`KismetMathLibrary.MakeColor` 0.0 1.0 1.0)))
    (:`2`
      (return (`KismetMathLibrary.MakeColor` 1.0 1.0)))
    (:`3`
      (return (`KismetMathLibrary.MakeColor` 0.5 0.0 1.0)))))

(fn `UI Create Game Result`
  (`/Engine/EditorBlueprintResources/StandardMacros.IsValid` (`self.WB_GameResult_Widget`)
    (:`Is Valid`
      _)
    (:`Is Not Valid`
      (bind _returnvalue (`|CreateWidget` "/Game/Merged/Widgets/WB_GameResult.WB_GameResult_C" self))
      (set `self.WB_GameResult_Widget` _returnvalue)))
  (`UserWidget.AddToViewport` (`self.WB_GameResult_Widget`) 0)
  (return))

(fn `UI_ShowLoadScreen`
  (params (LevelRowName :type Name))
  (`WidgetLayoutLibrary.RemoveAllWidgets`)
  (`/Engine/EditorBlueprintResources/StandardMacros.IsValid` (`self.WB_LoadScreen_Widget`)
    (:`Is Valid`
      _)
    (:`Is Not Valid`
      (bind _returnvalue (`|CreateWidget` "/Game/Merged/Widgets/WB_LoadScreen.WB_LoadScreen_C" self LevelRowName))
      (set `self.WB_LoadScreen_Widget` _returnvalue)))
  (`UserWidget.AddToViewport` (`self.WB_LoadScreen_Widget`) 0)
  (return))

(fn `UserConstructionScript`)