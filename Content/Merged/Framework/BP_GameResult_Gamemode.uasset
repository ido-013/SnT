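; Game mode for the multiplayer results level, placing each player's character at a start spot matching their final rank.
; Tick waits until all expected players connect and have profiles, indexing four PlayerStarts by numeric tag.
; It then spawns and possesses scaled characters, with None and Turtle falling back to Seahorse.
; Controller RPCs then set colors, fill every player's result widget with all standings, remove loading screens and set targets.
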(event `self.HandleStartingNewPlayer`
  (params (NewPlayer :type "PlayerController Object Reference"))
  (bind _asbp_game_result_player_controller (cast `/Game/Merged/Framework/BP_GameResult_PlayerController` NewPlayer))
  (`KismetArrayLibrary.Array_Add` (`self.All_ConnectedPlayers`) _asbp_game_result_player_controller)
  (`parent.HandleStartingNewPlayer` NewPlayer))

(event `self.ReceiveBeginPlay`
  (bind _asbp_shooter_gameinstance (cast `/Game/Merged/Framework/BP_Shooter_Gameinstance` (`GameplayStatics.GetGameInstance`)))
  (set `self.Num Connected Players` (`/Game/Merged/Framework/BP_Shooter_Gameinstance.Num Connected Players` _asbp_shooter_gameinstance)))

(event `self.ReceiveTick`
  (params (DeltaSeconds :type "Float (single-precision)"))
  (if (`self.IsAllPlayerGetProfile`)
    _
    (elif (== (`KismetArrayLibrary.Array_Length` (`self.All_ConnectedPlayers`)) (`self.Num Connected Players`))
      (bind _outactors (`GameplayStatics.GetAllActorsOfClass` "/Script/Engine.PlayerStart"))
      (if (== (`KismetArrayLibrary.Array_Length` _outactors) 4)
        (for _array_element _outactors
          (`KismetArrayLibrary.Array_Set` (`self.PlayerStarts`) (`KismetStringLibrary.Conv_StringToInt` (`KismetStringLibrary.Conv_NameToString` (`PlayerStart.PlayerStartTag` _array_element))) _array_element true))
        (set `self.IsAllPlayerGetProfile` true)
        (for _array_element_2 (`self.All_ConnectedPlayers`)
          (if (not (`/Game/Merged/Framework/BP_GameResult_PlayerController.IsPlayerProfile` _array_element_2))
            (set `self.IsAllPlayerGetProfile` false)))
        (if (`self.IsAllPlayerGetProfile`)
          (for _array_element_3 (`self.All_ConnectedPlayers`)
            (bind (_player_profile_info_player_name _player_profile_info_player_character _player_profile_info_player_record _player_profile_info_player_ranking) (break `/Game/Merged/SavedData/S_PlayerProfile` (`/Game/Merged/Framework/BP_GameResult_PlayerController.Player Profile Info` _array_element_3)))
            (`self.SpawnPlayerActor` _array_element_3 _player_profile_info_player_character _player_profile_info_player_ranking))
          (`self.Set_ActorColors`)
          (for _array_element_4 (`self.All_ConnectedPlayers`)
            (`/Game/Merged/Framework/BP_GameResult_PlayerController.RPC_SetDefault` _array_element_4)
            (`/Game/Merged/Framework/BP_GameResult_PlayerController.Create_GameResultWidget` _array_element_4)
            (for _array_element_5 (`self.All_ConnectedPlayers`)
              (bind (_player_profile_info_player_name_2 _player_profile_info_player_character_2 _player_profile_info_player_record_2 _player_profile_info_player_ranking_2 _player_profile_info_player_id) (break `/Game/Merged/SavedData/S_PlayerProfile` (`/Game/Merged/Framework/BP_GameResult_PlayerController.Player Profile Info` _array_element_5)))
              (`/Game/Merged/Framework/BP_GameResult_PlayerController.RPC_SetGameResultInfo` _array_element_4 _player_profile_info_player_name_2 _player_profile_info_player_ranking_2 _player_profile_info_player_record_2 _player_profile_info_player_id (`/Game/Merged/Framework/BP_GameResult_PlayerController.IsArrived` _array_element_5))))
          (for _array_element_6 (`self.All_ConnectedPlayers`)
            (`/Game/Merged/Framework/BP_GameResult_PlayerController.RPC_RemoveLoadScreen` _array_element_6)
            (`/Game/Merged/Framework/BP_GameResult_PlayerController.RPC_SetTargets` _array_element_6)))))))

(event `SpawnPlayerActor`
  (params (`Player Controller` :type "Controller Object Reference") (Character :type "/Game/Merged/SavedData/E_Characters Enum" :default "NewEnumerator0") (Rank :type Integer))
  (bind _playerstart (`self.ChoosePlayerStartPos` Rank))
  (`/Engine/EditorBlueprintResources/StandardMacros.IsValid` _playerstart
    (:`Is Valid`
      (`self.FuncSpawnActor` Character (`self.GetTransform` _playerstart) _playerstart `Player Controller`))))

(event `Set_ActorColors`
  (for _array_element (`self.All_ConnectedPlayers`)
    (`/Engine/EditorBlueprintResources/StandardMacros.IsValid` _array_element
      (:`Is Valid`
        (bind (_player_profile_info_player_name _player_profile_info_player_character _player_profile_info_player_record _player_profile_info_player_ranking _player_profile_info_player_id) (break `/Game/Merged/SavedData/S_PlayerProfile` (`/Game/Merged/Framework/BP_GameResult_PlayerController.Player Profile Info` _array_element)))
        (`/Game/Merged/Framework/BP_GameResult_PlayerController.RPC_SetPlayerActorColor` _array_element _player_profile_info_player_character _player_profile_info_player_id)))))

(fn `ChoosePlayerStartPos`
  (params (Rank :type Integer))
  (returns (PlayerStart :type "Actor Object Reference"))
  (bind _output_get (set `self.SelectedPlayerStart` (`|GetArrayItem` (`self.PlayerStarts`) Rank)))
  (return _output_get))

(fn `FuncSpawnActor`
  (params (Selection :type "/Game/Merged/SavedData/E_Characters Enum" :default "NewEnumerator0") (`Spawn Transform` :type "Transform Structure (by ref)") (`Start Spot` :type "Actor Object Reference") (`Player Controller` :type "Controller Object Reference"))
  (switch `/Game/Merged/SavedData/E_Characters` Selection
    (:`NewEnumerator0`
      (bind _returnvalue (`|SpawnActorFromClass` "/Game/Merged/Character/Seahorse/BP_Seahorse.BP_Seahorse_C" `Spawn Transform` "Undefined" "OverrideRootScale" null null :!label _label))
      (`self.SetActorScale3D` _returnvalue (`KismetMathLibrary.Conv_DoubleToVector` (`self.ActorScale`)))
      (`Controller.Possess` `Player Controller` _returnvalue)
      (`self.RestartPlayerAtPlayerStart` `Player Controller` `Start Spot`))
    (:`NewEnumerator1`
      (goto _label))
    (:`NewEnumerator2`
      (bind _returnvalue_2 (`|SpawnActorFromClass` "/Game/Merged/Character/Penguin/BP_Penguin.BP_Penguin_C" `Spawn Transform` "Undefined" "OverrideRootScale" null null))
      (`self.SetActorScale3D` _returnvalue_2 (`KismetMathLibrary.Conv_DoubleToVector` (`self.ActorScale`)))
      (`Controller.Possess` `Player Controller` _returnvalue_2)
      (`self.RestartPlayerAtPlayerStart` `Player Controller` `Start Spot`))
    (:`NewEnumerator3`
      (bind _returnvalue_3 (`|SpawnActorFromClass` "/Game/Merged/Character/Shark/BP_Shark.BP_Shark_C" `Spawn Transform` "Undefined" "OverrideRootScale" null null))
      (`self.SetActorScale3D` _returnvalue_3 (`KismetMathLibrary.Conv_DoubleToVector` (`self.ActorScale`)))
      (`Controller.Possess` `Player Controller` _returnvalue_3)
      (`self.RestartPlayerAtPlayerStart` `Player Controller` `Start Spot`))
    (:`NewEnumerator4`
      (goto _label)))
  (return))

(fn `UserConstructionScript`)