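; Menu game mode that runs the solo and multiplayer lobbies, branching on login by game instance mode and current map.
; It tracks connected menu controllers, assigns index-based player IDs and ends sessions for overflow joiners.
; Server events loop over controllers to push names, characters, level selection, room name and ready states, with the first player excluded from the all-ready check.
; It also passes the map to the game state and updates the session's IsRacing setting.
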(event `self.K2_OnLogout`
  (params (ExitingController :type "Controller Object Reference"))
  (bind _asbp_menu_controller (cast `/Game/Merged/Framework/BP_MenuController` ExitingController))
  (`KismetArrayLibrary.Array_RemoveItem` (`self.All_ConnectedPlayers`) _asbp_menu_controller)
  (`self.UpdateLobby` true true)
  (`self.Server_UpdateReadyState`))

(event `self.K2_PostLogin`
  (params (NewPlayer :type "PlayerController Object Reference"))
  (bind _all_connectedplayers (`self.All_ConnectedPlayers`))
  (bind _asbp_shooter_gameinstance (cast `/Game/Merged/Framework/BP_Shooter_Gameinstance` (`GameplayStatics.GetGameInstance`)))
  (if (`/Game/Merged/Framework/BP_Shooter_Gameinstance.IsSoloGame` _asbp_shooter_gameinstance)
    ;[1 1 1] Lobby Only
    (bind _returnvalue (`GameplayStatics.GetCurrentLevelName` true))
    (switch `string` _returnvalue
      (:`SoloLobbyMenu_Map`
        (bind _asbp_menu_controller (cast `/Game/Merged/Framework/BP_MenuController` NewPlayer))
        (`/Game/Merged/Framework/BP_MenuController.CreateSoloLobbyMenu` _asbp_menu_controller)))
    (elif (<= (`KismetArrayLibrary.Array_Length` (`self.All_ConnectedPlayers`)) 4)
      ;[1 1 1] Lobby Only
      (bind _returnvalue_2 (`GameplayStatics.GetCurrentLevelName` true))
      (switch `string` _returnvalue_2
        (:`LobbyMenu_Map`
          (if (`KismetSystemLibrary.IsServer`)
            (`self.Server_SetIsRacing` false))
          (bind _asbp_menu_controller_2 (cast `/Game/Merged/Framework/BP_MenuController` NewPlayer))
          (`KismetArrayLibrary.Array_Add` _all_connectedplayers _asbp_menu_controller_2)
          (set `/Game/Merged/Framework/BP_MenuController.IsReady` false _asbp_menu_controller_2)
          (`/Game/Merged/Framework/BP_MenuController.CreateLobbyMenu` _asbp_menu_controller_2)
          (bind _availableid (`self.GetPlayerId` _all_connectedplayers))
          (`/Game/Merged/Framework/BP_MenuController.Initial_Setup` _asbp_menu_controller_2 _availableid)
          (bind _asbp_shooter_gameinstance_2 (cast `/Game/Merged/Framework/BP_Shooter_Gameinstance` (`GameplayStatics.GetGameInstance`)))
          (`/Game/Merged/Framework/BP_MenuController.UpdateRoomInfo` _asbp_menu_controller_2 (`KismetTextLibrary.Conv_StringToText` (`/Game/Merged/Framework/BP_Shooter_Gameinstance.Room Name` _asbp_shooter_gameinstance_2)))
          (if (>= (`KismetArrayLibrary.Array_Length` (`self.All_ConnectedPlayers`)) 4)
            (`self.UpdateLobby` false true))))
      (else
        (bind _asbp_menu_controller_3 (cast `/Game/Merged/Framework/BP_MenuController` NewPlayer))
        (`/Game/Merged/Framework/BP_MenuController.EndClientSession` _asbp_menu_controller_3)))))

(event `UpdateLobby`
  (params (PlayerInfos :type Boolean) (LevelSelection :type Boolean))
  (bind _all_playerprofiles (`self.All_PlayerProfiles`))
  (if PlayerInfos
    (`KismetArrayLibrary.Array_Clear` (`self.All_PlayerProfiles`))
    (for _array_element (`self.All_ConnectedPlayers`)
      (`KismetArrayLibrary.Array_Add` (`self.All_PlayerProfiles`) (`/Game/Merged/Framework/BP_MenuController.PlayerProfileInfo` _array_element))))
  (for _array_element_2 (`self.All_ConnectedPlayers`)
    (if PlayerInfos
      (`/Game/Merged/Framework/BP_MenuController.UpdatePlayerNames` _array_element_2 _all_playerprofiles)
      (`/Game/Merged/Framework/BP_MenuController.UpdatePlayerCharacters` _array_element_2 _all_playerprofiles))
    (if LevelSelection
      (`/Game/Merged/Framework/BP_MenuController.UpdateLevelSelection` _array_element_2 (`self.SelectedLevelName`)))))

(event `Server_SetMapDataRowName`
  (bind _asbp_general_game_state (cast `/Game/Merged/Framework/BP_General_GameState` (`GameplayStatics.GetGameState`))
    (:`then`
      (`/Game/Merged/Framework/BP_General_GameState.Set_MapDataRowName` _asbp_general_game_state (`self.SelectedLevelName`)))
    (:`CastFailed`
      (`KismetSystemLibrary.PrintString` "Failed To CastGeneral_GameState"))))

(event `Server_SavePlayerProfileForInstance`
  (for _array_element (`self.All_ConnectedPlayers`)
    (`/Game/Merged/Framework/BP_MenuController.SavePlayerProfileForInstance` _array_element)))

(event `UpdateCharacters`
  (`KismetArrayLibrary.Array_Clear` (`self.All_PlayerProfiles`))
  (for _array_element (`self.All_ConnectedPlayers`)
    (bind _playerprofileinfo (`/Game/Merged/Framework/BP_MenuController.PlayerProfileInfo` _array_element))
    (`KismetArrayLibrary.Array_Add` (`self.All_PlayerProfiles`) _playerprofileinfo)
    (bind (_player_name _player_character _player_record _player_ranking _player_id) (break `/Game/Merged/SavedData/S_PlayerProfile` _playerprofileinfo))
    (`KismetSystemLibrary.PrintString` (`KismetStringLibrary.Concat_StrStr` (`KismetStringLibrary.Conv_IntToString` _player_id) (`|GetEnumeratorNameAsString` _player_character))))
  (for _array_element_2 (`self.All_ConnectedPlayers`)
    (`/Game/Merged/Framework/BP_MenuController.UpdatePlayerCharacters` _array_element_2 (`self.All_PlayerProfiles`))))

(event `SetIsReady`
  (params (PID :type Integer) (IsReady :type Boolean))
  (for _array_element (`self.All_ConnectedPlayers`)
    (bind (_playerprofileinfo_player_name _playerprofileinfo_player_character _playerprofileinfo_player_record _playerprofileinfo_player_ranking _playerprofileinfo_player_id) (break `/Game/Merged/SavedData/S_PlayerProfile` (`/Game/Merged/Framework/BP_MenuController.PlayerProfileInfo` _array_element)))
    (if (== _playerprofileinfo_player_id PID)
      (set `/Game/Merged/Framework/BP_MenuController.IsReady` IsReady _array_element))))

(event `SetPlayerCharacter`
  (params (PID :type Integer) (`Player Profile Info Player Character` :type "/Game/Merged/SavedData/E_Characters Enum" :default "NewEnumerator0"))
  (for _array_element (`self.All_ConnectedPlayers`)
    (bind (_playerprofileinfo_player_name _playerprofileinfo_player_character _playerprofileinfo_player_record _playerprofileinfo_player_ranking _playerprofileinfo_player_id) (break `/Game/Merged/SavedData/S_PlayerProfile` (`/Game/Merged/Framework/BP_MenuController.PlayerProfileInfo` _array_element)))
    (if (== _playerprofileinfo_player_id PID)
      (set `/Game/Merged/Framework/BP_MenuController.PlayerProfileInfo` (make `/Game/Merged/SavedData/S_PlayerProfile` _playerprofileinfo_player_name `Player Profile Info Player Character` _playerprofileinfo_player_record _playerprofileinfo_player_ranking _playerprofileinfo_player_id) _array_element)
      (`/Game/Merged/Framework/BP_MenuController.SavePlayerProfileForInstance` _array_element))))

(event `Server_SetIsRacing`
  (params (IsRacing :type Boolean))
  (bind (_numconnections _numprivateconnections _bislan _bisdedicated _ballowinvites _ballowjoininprogress _bisanticheatenabled _builduniqueid _extrasettings) (`AdvancedSessionsLibrary.GetSessionSettings`)
    (:`OnSuccess`
      (for _array_element _extrasettings
        (bind _returnvalue (`AdvancedSessionsLibrary.GetSessionPropertyKey` _array_element))
        (if (== _returnvalue "IsRacing")
          (`|VariableSetRef` _array_element (`AdvancedSessionsLibrary.MakeLiteralSessionPropertyInt` "IsRacing" (`KismetMathLibrary.Conv_BoolToInt` IsRacing))))
        (`KismetArrayLibrary.Array_AddUnique` (`self.Settings`) _array_element))
      (bind _modifiedsettingsarray (`AdvancedSessionsLibrary.AddOrModifyExtraSettings` _extrasettings (`self.Settings`)))
      (`UpdateSessionCallbackProxyAdvanced.UpdateSession` _modifiedsettingsarray _numconnections _numprivateconnections _bislan _ballowinvites _ballowjoininprogress true _bisdedicated
        (:`OnSuccess`
          (`KismetSystemLibrary.PrintString` "Update session!"))
        (:`OnFailure`
          (`KismetSystemLibrary.PrintString` "Failed Update Session"))))
    (:`OnFailure`
      (`KismetSystemLibrary.PrintString` "Failed to get session settings"))))

(event `UpdateRoomInfo`
  (for _array_element (`self.All_ConnectedPlayers`)
    (bind _asbp_shooter_gameinstance (cast `/Game/Merged/Framework/BP_Shooter_Gameinstance` (`GameplayStatics.GetGameInstance`)))
    (`/Game/Merged/Framework/BP_MenuController.UpdateRoomInfo` _array_element (`KismetTextLibrary.Conv_StringToText` (`/Game/Merged/Framework/BP_Shooter_Gameinstance.Room Name` _asbp_shooter_gameinstance)))))

(event `Server_UpdateReadyState`
  (`self.GetPlayerReadyStates`)
  (`KismetArrayLibrary.Array_Clear` (`self.ReadyStates`))
  (set `self.ReadyStates` (`|MakeArray` 0 0 0 0))
  (for _array_element (`self.All_ConnectedPlayers`)
    (bind (_playerprofileinfo_player_name _playerprofileinfo_player_character _playerprofileinfo_player_record _playerprofileinfo_player_ranking _playerprofileinfo_player_id) (break `/Game/Merged/SavedData/S_PlayerProfile` (`/Game/Merged/Framework/BP_MenuController.PlayerProfileInfo` _array_element)))
    (`KismetArrayLibrary.Array_Set` (`self.ReadyStates`) _playerprofileinfo_player_id (`KismetMathLibrary.Conv_BoolToInt` (`/Game/Merged/Framework/BP_MenuController.IsReady` _array_element)))
    (for _array_element_2 (`self.All_ConnectedPlayers`) :!label _label
      (`/Game/Merged/Framework/BP_MenuController.Update_PlayerReadyState` _array_element_2 (`self.ReadyStates`))))
  (goto _label))

(fn `GetPlayerId`
  (params (Array :type "Array of /Game/Merged/Framework/BP_MenuController Object Reference"))
  (returns (AvailableId :type Integer))
  (locals (Id :type Integer :default 1) (IsFindAvailableId :type Boolean :default true))
  (return (`KismetArrayLibrary.Array_LastIndex` Array)))

(fn `GetPlayerReadyStates`
  (locals (IsReady :type Boolean :default true))
  (for (_array_element _array_index) (`self.All_ConnectedPlayers`)
    (if (!= _array_index 0)
      (if (not (`/Game/Merged/Framework/BP_MenuController.IsReady` _array_element))
        (set `local.IsReady` false))))
  (if (`local.IsReady`)
    (set `self.IsReadyAllPlayer` true)
    (else
      (set `self.IsReadyAllPlayer` false))))

(fn `UserConstructionScript`)