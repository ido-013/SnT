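; Player controller for the multiplayer menu and lobby, handling UI-only input, lobby and load screen widgets, and session exit to the main menu.
; Initial setup loads the saved player profile, creating it if missing, and sends it to the server, which asks BP_Menu_Gamemode to update the lobby.
; Controller events pass room name, player names and level selection to the cached lobby widget.
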(event `CreateLoadScreen`
  (params (CurrLevelRowName :type Name))
  (`self.UI_ShowLoadScreen` CurrLevelRowName))

(event `self.ReceiveBeginPlay`
  (if (`self.IsLocalController`)
    (set `self.bShowMouseCursor` true)
    (`WidgetBlueprintLibrary.SetInputMode_UIOnlyEx` self null)))

(event `EndClientSession`
  (`DestroySessionCallbackProxy.DestroySession` self
    (:`then`
      (`GameplayStatics.OpenLevel` "MainMenu_Map"))))

(event `CreateLobbyMenu`
  (`self.UI_ShowLobbyMenu`))

(event `UpdateRoomInfo`
  (params (S_PlayerProfile :type "/Game/Merged/SavedData/S_PlayerProfile Structure (by ref)"))
  (`/Game/Merged/Widgets/WB_LobbyMenu.UpdateRoomName` (`self.WB_LobbyMenu_Widget`) (`.Player_Name_3_7DE3D9AD43B26C512D8954ADA2D53F0D` (break `/Game/Merged/SavedData/S_PlayerProfile` S_PlayerProfile))))

(event `UpdatePlayerNames`
  (params (PlayerProfiles :type "Array of /Game/Merged/SavedData/S_PlayerProfile Structure"))
  (bind _wb_lobbymenu_widget (`self.WB_LobbyMenu_Widget`))
  (`/Engine/EditorBlueprintResources/StandardMacros.IsValid` _wb_lobbymenu_widget
    (:`Is Valid`
      (`/Game/Merged/Widgets/WB_LobbyMenu.ClearPlayerNames` _wb_lobbymenu_widget)
      (`/Game/Merged/Widgets/WB_LobbyMenu.UpdatePlayerNames` _wb_lobbymenu_widget PlayerProfiles))))

(event `Initial_Setup`
  (`self.LoadSavedProfile`)
  (`self.Server_UpdateLobby` (`self.PlayerProfileInfo`)))

(event `Server_UpdateLobby`
  (params (PlayerProfile :type "/Game/Merged/SavedData/S_PlayerProfile Structure"))
  (set `self.PlayerProfileInfo` PlayerProfile)
  (if (`KismetSystemLibrary.IsServer`)
    (`KismetSystemLibrary.PrintString` "It's Server!")
    (bind _asbp_menu_gamemode (cast `/Game/Merged/Framework/BP_Menu_Gamemode` (`GameplayStatics.GetGameMode`))
      (:`then`
        (`/Game/Merged/Framework/BP_Menu_Gamemode.UpdateLobby` _asbp_menu_gamemode true true))
      (:`CastFailed`
        (`KismetSystemLibrary.PrintString` "Game Mode Cast Failed")))
    (else
      (`KismetSystemLibrary.PrintString` "It's Not Server!"))))

(event `RPC_UpdateLevelSelection`
  (params (LevelRowName :type Name))
  (bind _wb_lobbymenu_widget (`self.WB_LobbyMenu_Widget`))
  (`/Engine/EditorBlueprintResources/StandardMacros.IsValid` _wb_lobbymenu_widget
    (:`Is Valid`
      (`/Game/Merged/Widgets/WB_LobbyMenu.UpdateLevelSelection` _wb_lobbymenu_widget LevelRowName))))

(fn `LoadSavedProfile`
  (locals (Lcl_SlotName :type String :default "PlayerProfile_Slot"))
  (bind _returnvalue (`GameplayStatics.DoesSaveGameExist` (`local.Lcl_SlotName`)))
  (if (not _returnvalue)
    (bind _returnvalue_2 (`GameplayStatics.CreateSaveGameObject` "/Game/Merged/SavedData/SG_PlayerProfile.SG_PlayerProfile_C"))
    (`GameplayStatics.SaveGameToSlot` _returnvalue_2 (`local.Lcl_SlotName`)))
  (bind _returnvalue_3 (`GameplayStatics.LoadGameFromSlot` (`local.Lcl_SlotName`)))
  (bind _assg_player_profile (cast `/Game/Merged/SavedData/SG_PlayerProfile` _returnvalue_3))
  (set `self.PlayerProfileInfo` (`/Game/Merged/SavedData/SG_PlayerProfile.PlayerProfile` _assg_player_profile))
  (return))

(fn `UI_ShowLoadScreen`
  (params (LevelRowName :type Name))
  (`WidgetLayoutLibrary.RemoveAllWidgets`)
  (`/Engine/EditorBlueprintResources/StandardMacros.IsValid` (`self.WB_LoadScreen_Widget`)
    (:`Is Valid`
      _)
    (:`Is Not Valid`
      (bind _returnvalue (`|CreateWidget` "/Game/Merged/Widgets/WB_LoadScreen.WB_LoadScreen_C" self LevelRowName))
      (set `self.WB_LoadScreen_Widget` _returnvalue)))
  (`UserWidget.AddToViewport` (`self.WB_LoadScreen_Widget`) 0)
  (return))

(fn `UI_ShowLobbyMenu`
  (`/Engine/EditorBlueprintResources/StandardMacros.IsValid` (`self.WB_LobbyMenu_Widget`)
    (:`Is Valid`
      _)
    (:`Is Not Valid`
      (bind _returnvalue (`|CreateWidget` "/Game/Merged/Widgets/WB_LobbyMenu.WB_LobbyMenu_C" self))
      (set `self.WB_LobbyMenu_Widget` _returnvalue)))
  (`UserWidget.AddToViewport` (`self.WB_LobbyMenu_Widget`) 0)
  (return))

(fn `UserConstructionScript`)