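; BP_PenguinProj is the penguin player's bouncing projectile, which can stun the player who owns it.
; Tick runs a lifetime timer that switches Pawn collision to Block shortly after spawn and destroys the actor at MaxDestroyTimer.
; Hits on anything but the owner reflect velocity off the surface normal.
; After a half-second grace period, hitting the owner calls StunEvent on BP_Player and expires the timer.
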(event `self.ReceiveBeginPlay`
  (set `self.MyOwner` (`self.GetOwner`)))

(event `self.Sphere.OnComponentHit`
  (params (HitComponent :type "PrimitiveComponent Object Reference") (OtherActor :type "Actor Object Reference") (OtherComp :type "PrimitiveComponent Object Reference") (NormalImpulse :type "Vector Structure") (Hit :type "HitResult Structure (by ref)"))
  (bind _projectilemovement (`self.ProjectileMovement`))
  (if (== OtherActor (`self.MyOwner`))
    (if (> (`self.DestroyTimer`) 0.5)
      (switch `ECollisionChannel` (`PrimitiveComponent.GetCollisionObjectType` (`self.GetComponentByClass` OtherActor "/Script/Engine.PrimitiveComponent"))
        (:`ECC_Pawn`
          (bind _asbp_player (cast `/Game/Merged/Player/BP_Player` OtherActor))
          (`/Game/Merged/Player/BP_Player.StunEvent` _asbp_player 0.8 1.5 10 2.0)
          (set `self.DestroyTimer` (`self.MaxDestroyTimer`)))))
    (else
      (set `MovementComponent.Velocity` (`KismetMathLibrary.GetReflectionVector` (`MovementComponent.Velocity` _projectilemovement) (`.Normal` (`GameplayStatics.BreakHitResult` Hit))) _projectilemovement))))

(event `self.ReceiveTick`
  (params (DeltaSeconds :type "Float (single-precision)"))
  (bind _output_get (set `self.DestroyTimer` (+ DeltaSeconds (`self.DestroyTimer`))))
  (if (> _output_get 0.05)
    (`PrimitiveComponent.SetCollisionResponseToChannel` (`self.Sphere`) "ECC_Pawn" "ECR_Block")
    (if (> _output_get (`self.MaxDestroyTimer`))
      (`self.K2_DestroyActor`))))

(fn `UserConstructionScript`)