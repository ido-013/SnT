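; Seahorse projectile that grows and slows in flight, then stops on the first actor it overlaps.
; Each tick until that overlap, Set Projectile Attr enlarges the sphere and damps velocity while speed stays above set limits.
; Overlapping a Player-tagged actor prints a stun message and destroys it; otherwise a lifetime timer removes it.
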(event `self.ReceiveActorBeginOverlap`
  (params (OtherActor :type "Actor Object Reference"))
  (set `MovementComponent.Velocity` (0.0 0.0 0.0) (`self.ProjectileMovement`))
  (set `self.IsAttached` true)
  (if (`self.ActorHasTag` OtherActor "Player")
    (`KismetSystemLibrary.PrintString` "Player Stun" true true (struct :`R` 0.578125 :`B` 0.004 :`A` 1.0))
    (`self.K2_DestroyActor`)))

(event `self.ReceiveTick`
  (params (DeltaSeconds :type "Float (single-precision)"))
  (bind _output_get (set `self.DestroyTimer` (+ DeltaSeconds (`self.DestroyTimer`))))
  (if (> _output_get (`self.MaxDestroyTimer`))
    (`self.K2_DestroyActor`)
    (elif (not (`self.IsAttached`))
      (`self.Set Projectile Attr` 50.0 0.02 10.0 0.99))))

(fn `UserConstructionScript`)