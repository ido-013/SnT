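; BP_TrackingRange is an obstacle detection zone that steers the homing projectile movement of its Tracking object.
; Overlapping characters join a list, and the projectile homes on the first one's mesh.
; On exit the list shrinks to the player count, retargeting its first entry or Sphere1 when empty.
; With nobody inside, a Tick timer periodically alternates the target between Sphere1 and Sphere2, creating a patrol.
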(event `self.ReceiveBeginPlay`
  (set `self.HowManyPlayer` 0)
  (set `self.SphereSwitch` true))

(event `self.ReceiveTick`
  (params (DeltaSeconds :type "Float (single-precision)"))
  (bind _output_get (set `self.TrackTimer` (+ DeltaSeconds (`self.TrackTimer`))))
  (if (== (`self.HowManyPlayer`) 0)
    (if (>= _output_get 3.0)
      (set `self.TrackTimer` 0.0)
      (if (`self.SphereSwitch`)
        (set `ProjectileMovementComponent.HomingTargetComponent` (`self.Sphere1`) (`/Game/Merged/Obstacles/BP_Tracking.ProjectileMovement` (`self.Tracking`)))
        (set `self.SphereSwitch` false)
        (else
          (set `ProjectileMovementComponent.HomingTargetComponent` (`self.Sphere2`) (`/Game/Merged/Obstacles/BP_Tracking.ProjectileMovement` (`self.Tracking`)))
          (set `self.SphereSwitch` true))))))

(event `self.Sphere.OnComponentBeginOverlap`
  (params (OverlappedComponent :type "PrimitiveComponent Object Reference") (OtherActor :type "Actor Object Reference") (OtherComp :type "PrimitiveComponent Object Reference") (OtherBodyIndex :type Integer) (bFromSweep :type Boolean) (SweepResult :type "HitResult Structure (by ref)"))
  (bind _asbp_character (cast `/Game/Merged/Character/BP_Character` OtherActor))
  (`KismetArrayLibrary.Array_Add` (`self.PlayerList`) _asbp_character)
  (set `self.HowManyPlayer` (+ (`self.HowManyPlayer`) 1))
  (set `ProjectileMovementComponent.HomingTargetComponent` (`Character.Mesh` (`|GetArrayItem` (`self.PlayerList`))) (`/Game/Merged/Obstacles/BP_Tracking.ProjectileMovement` (`self.Tracking`))))

(event `self.Sphere.OnComponentEndOverlap`
  (params (OverlappedComponent :type "PrimitiveComponent Object Reference") (OtherActor :type "Actor Object Reference") (OtherComp :type "PrimitiveComponent Object Reference") (OtherBodyIndex :type Integer))
  (cast `/Game/Merged/Character/BP_Character` OtherActor)
  (bind _output_get (set `self.HowManyPlayer` (- (`self.HowManyPlayer`) 1)))
  (`KismetArrayLibrary.Array_RemoveItem` (`self.PlayerList`))
  (`KismetArrayLibrary.Array_Resize` (`self.PlayerList`) _output_get)
  (if (> _output_get 0)
    (set `ProjectileMovementComponent.HomingTargetComponent` (`Character.Mesh` (`|GetArrayItem` (`self.PlayerList`))) (`/Game/Merged/Obstacles/BP_Tracking.ProjectileMovement` (`self.Tracking`)))
    (else
      (set `ProjectileMovementComponent.HomingTargetComponent` (`self.Sphere1`) (`/Game/Merged/Obstacles/BP_Tracking.ProjectileMovement` (`self.Tracking`))))))

(fn `UserConstructionScript`)