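; Race track manager that acts as the finish trigger and runs the start and end countdowns through BP_Shooter_Gamemode's match state.
; Overlap starts the end count, ends racing for the player and marks their controller as arrived.
; Tick advances the countdown text and match state, cutting it short once all have arrived.
; BeginPlay builds a table of remaining distance from each checkpoint to this actor, summing squared segment lengths.
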(event `self.ReceiveActorBeginOverlap`
  (params (OtherActor :type "Actor Object Reference"))
  (bind _matchstate (`self.Get_MatchState`))
  (if (not (`|EnumEquality` _matchstate "NewEnumerator2"))
    (set `self.CountSeconds` 0.0)
    (`self.Set_MatchState` "NewEnumerator2"))
  (bind _asbp_player (cast `/Game/Merged/Character/Player/BP_Player` OtherActor))
  (`/Game/Merged/Character/Player/BP_Player.EndRacing` _asbp_player)
  (`self.Get_MatchTime`)
  (bind _asbp_shooter_player_controller (cast `/Game/Merged/Framework/BP_Shooter_PlayerController` (`self.GetInstigatorController` OtherActor)))
  (`/Game/Merged/Framework/BP_Shooter_PlayerController.SetRetired` _asbp_shooter_player_controller false)
  (set `/Game/Merged/Framework/BP_Shooter_PlayerController.IsArrived` true _asbp_shooter_player_controller))

(event `self.ReceiveBeginPlay`
  (set `self.CountSeconds` 0.0)
  (bind _outactors (`GameplayStatics.GetAllActorsOfClass` "/Game/Merged/Track/BP_Checkpoint.BP_Checkpoint_C"))
  (set `self.Checkpoints` _outactors)
  (`self.Calculate Checkpoint Distance`))

(event `self.ReceiveTick`
  (params (DeltaSeconds :type "Float (single-precision)"))
  (set `self.DeltaSeconds` DeltaSeconds)
  (bind _matchstate (`self.Get_MatchState`))
  (switch `/Game/Merged/Track/E_MatchState` _matchstate
    (:`NewEnumerator1`
      (bind _asbp_shooter_gamemode (`self.Get_ShooterGamemode`))
      (`/Game/Merged/Framework/BP_Shooter_Gamemode.CreateCountdownScreen` _asbp_shooter_gamemode)
      (`/Game/Merged/Framework/BP_Shooter_Gamemode.VisibleCountdown` _asbp_shooter_gamemode "Visible")
      (`self.CountDownFunc` "NewEnumerator4" 3.0 "Go!")
      (set `/Game/Merged/Framework/BP_Shooter_Gamemode.IsRacing` true _asbp_shooter_gamemode)
      (`KismetSystemLibrary.Delay` 2.0)
      (`/Game/Merged/Framework/BP_Shooter_Gamemode.VisibleCountdown` _asbp_shooter_gamemode "Hidden"))
    (:`NewEnumerator2`
      (bind _asbp_shooter_gamemode_2 (`self.Get_ShooterGamemode`))
      (`/Game/Merged/Framework/BP_Shooter_Gamemode.VisibleCountdown` _asbp_shooter_gamemode_2 "Visible")
      (`self.CountDownFunc` "NewEnumerator3" 10.0 "Finish!")
      (`KismetSystemLibrary.Delay` 3.0)
      (`/Game/Merged/Framework/BP_Shooter_Gamemode.VisibleCountdown` _asbp_shooter_gamemode_2 "Hidden")
      (set `/Game/Merged/Framework/BP_Shooter_Gamemode.IsRacing` false _asbp_shooter_gamemode_2))))

(fn `Calculate DIstance`
  (params (Index :type Integer))
  (returns (Distance :type "Float (double-precision)"))
  (bind _output (`|GetArrayItem` (`self.Checkpoints`) Index))
  (bind _returnvalue (`self.K2_GetActorLocation` _output))
  (bind _nextcheckpoint (`/Game/Merged/Track/BP_Checkpoint.NextCheckpoint` _output))
  (`/Engine/EditorBlueprintResources/StandardMacros.IsValid` _nextcheckpoint
    (:`Is Valid`
      (return (`KismetMathLibrary.Vector_DistanceSquared` _returnvalue (`self.K2_GetActorLocation` _nextcheckpoint))))
    (:`Is Not Valid`
      (return (`KismetMathLibrary.Vector_DistanceSquared` _returnvalue (`self.K2_GetActorLocation` (`|GetArrayItem` (`self.Checkpoints`) (+ Index 1))))))))

(fn `CountDownFunc`
  (params (TargetState :type "/Game/Merged/Track/E_MatchState Enum" :default "NewEnumerator0") (CountDownSeconds :type "Float (double-precision)") (LastText :type Text))
  (bind _asbp_shooter_gamemode (`self.Get_ShooterGamemode`))
  (if (`/Game/Merged/Framework/BP_Shooter_Gamemode.Is All Arrived` _asbp_shooter_gamemode)
    (`self.Set_MatchState` TargetState :!label _label)
    (bind _asbp_shooter_gamemode_2 (`self.Get_ShooterGamemode`))
    (`/Game/Merged/Framework/BP_Shooter_Gamemode.SetTextCountdown` _asbp_shooter_gamemode_2 LastText)
    (else
      (bind _output_get (set `self.CountSeconds` (+ (`self.CountSeconds`) (`self.DeltaSeconds`))))
      (if (< _output_get CountDownSeconds)
        (bind _output_get_2 (set `/Game/Merged/Framework/BP_Shooter_Gamemode.CountDownNum` (- CountDownSeconds (`KismetMathLibrary.FTrunc` (`self.CountSeconds`))) _asbp_shooter_gamemode))
        (`/Game/Merged/Framework/BP_Shooter_Gamemode.SetTextCountdown` _asbp_shooter_gamemode (`KismetTextLibrary.Conv_IntToText` _output_get_2))
        (else
          (goto _label))))))

(fn `UserConstructionScript`)