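; BP_Checkpoint is a track checkpoint trigger that reports to AI and characters passing through, with its cube hidden at play.
; Box overlap start stores the actor's IsForward result and calls UpdateIndex on BP_AI actors.
; Overlap end calls BP_Character's UpdateCheckpoint only if that result has flipped, filtering out back-outs.
; GetIsForward contains a forward-vector dot-product side test, shown as unconnected nodes.
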(event `self.ReceiveBeginPlay`
  (`SceneComponent.SetVisibility` (`self.Cube`) false false))

(event `self.Box.OnComponentBeginOverlap`
  (params (OverlappedComponent :type "PrimitiveComponent Object Reference") (OtherActor :type "Actor Object Reference") (OtherComp :type "PrimitiveComponent Object Reference") (OtherBodyIndex :type Integer) (bFromSweep :type Boolean) (SweepResult :type "HitResult Structure (by ref)"))
  (set `self.IsForward` (`self.Get IsForward` OtherActor))
  (bind _asbp_ai (cast `/Game/Merged/Character/AI/BP_AI` OtherActor))
  (`/Game/Merged/Character/AI/BP_AI.Update Index` _asbp_ai self))

(event `self.Box.OnComponentEndOverlap`
  (params (OverlappedComponent :type "PrimitiveComponent Object Reference") (OtherActor :type "Actor Object Reference") (OtherComp :type "PrimitiveComponent Object Reference") (OtherBodyIndex :type Integer))
  (if (xor (`self.Get IsForward` OtherActor) (`self.IsForward`))
    (bind _asbp_character (cast `/Game/Merged/Character/BP_Character` OtherActor))
    (`/Game/Merged/Character/Player/BP_Player.Update Checkpoint` _asbp_character self)))

(fn `UserConstructionScript`)