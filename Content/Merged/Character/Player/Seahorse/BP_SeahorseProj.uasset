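; BP_SeahorseProj is the seahorse character's projectile, which stuns players it hits and expires on a timer.
; Tick starts blocking Pawns once the timer is positive, then grows the sphere and damps velocity while speed exceeds a threshold.
; Hits ignore the owner briefly; Pawn hits call StunEvent on BP_Player and force expiry, while Knockback-type objects stop the projectile.
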(event `self.ReceiveBeginPlay`
  (set `self.MyOwner` (`self.GetOwner`)))

(event `self.ReceiveHit`
  (params (MyComp :type "PrimitiveComponent Object Reference") (Other :type "Actor Object Reference") (OtherComp :type "PrimitiveComponent Object Reference") (bSelfMoved :type Boolean) (HitLocation :type "Vector Structure") (HitNormal :type "Vector Structure") (NormalImpulse :type "Vector Structure") (Hit :type "HitResult Structure (by ref)"))
  (if (== Other (`self.MyOwner`))
    (if (> (`self.DestroyTimer`) 0.5)
      (switch `ECollisionChannel` (`PrimitiveComponent.GetCollisionObjectType` (`self.GetComponentByClass` Other "/Script/Engine.PrimitiveComponent")) :!label _label
        (:`ECC_Pawn`
          (bind _asbp_player (cast `/Game/Merged/Character/Player/BP_Player` Other))
          (`/Game/Merged/Character/Player/BP_Player.StunEvent` _asbp_player 0.8 1.5 10 2.0)
          (set `self.DestroyTimer` (`self.MaxDestroyTimer`)))
        (:`ECC_GameTraceChannel3`
          (set `MovementComponent.Velocity` (0.0 0.0 0.0) (`self.ProjectileMovement`)))))
    (else
      (goto _label))))

(event `self.ReceiveTick`
  (params (DeltaSeconds :type "Float (single-precision)"))
  (bind _output_get (set `self.DestroyTimer` (+ DeltaSeconds (`self.DestroyTimer`))))
  (if (> _output_get 0.0)
    (`PrimitiveComponent.SetCollisionResponseToChannel` (`self.Sphere`) "ECC_Pawn" "ECR_Block")
    (if (> _output_get (`self.MaxDestroyTimer`))
      (`self.K2_DestroyActor`)
      (else
        (`self.Set Projectile Attr` 50.0 0.03 0.99)))))

(fn `UserConstructionScript`)