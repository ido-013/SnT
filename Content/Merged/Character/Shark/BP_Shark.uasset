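; Shark character Blueprint whose skill input triggers a bite lunge through a server RPC that calls a second RPC.
; That RPC adds a CharacterMovement force toward the Endpos component's location, gated by cooldown and biting flags.
; Neither flag is reset by live logic, and nothing is spawned despite the RPC names.
; A timed, swept lerp that would move the shark and end the bite is disconnected from Tick.
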(event `EnhancedInput|/Game/Merged/Character/Player/Input/Actions/IA_Skill`
  (params (ActionValue :type Boolean) (ElapsedSeconds :type "Float (double-precision)") (TriggeredSeconds :type "Float (double-precision)") (InputAction :type "InputAction Object Reference" :default "/Game/Merged/Character/Player/Input/Actions/IA_Skill.IA_Skill"))
  (:`Started`
    (`self.RPC_Server_SpawnActor_Shark`)))

(event `RPC_Server_SpawnActor_Shark`
  (`self.RPC_SpawnActor_Shark`)
  (set `self.MoveSpeed` 15.0)
  (set `self.BiteStartTime` 0.0)
  (set `self.BiteDuration` 1.0))

(event `RPC_SpawnActor_Shark`
  (if (not (`self.IsCooldown`))
    (set `self.IsCooldown` true)
    (if (not (`self.isBiting`))
      (set `self.isBiting` true)
      (bind _output_get (set `self.StartLocation` (`self.K2_GetActorLocation`)))
      (bind _output_get_2 (set `self.MoveDistance` (`SceneComponent.K2_GetComponentLocation` (`self.Endpos`))))
      (`CharacterMovementComponent.AddForce` (`self.CharacterMovement`) (* (`self.Force`) (`KismetMathLibrary.Normal` (- _output_get_2 _output_get)))))))

(event `self.ReceiveTick`
  (params (DeltaSeconds :type "Float (single-precision)"))
  (`parent.ReceiveTick` DeltaSeconds)
  (if (`self.isBiting`)
    _))

(fn `UserConstructionScript`)