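; AI racer character that follows BP_AITrack checkpoints in a loop by steering its ProjectileMovement homing target.
; A forward line trace detects obstacles, then a grid of capsule traces picks a clear point near the target and spawns a stopover as temporary homing target.
; UpdateIndex advances checkpoints and clears stopovers, while ResetTarget restores the saved target.
; Tick also drives max speed from gauge-based dashing, disabled while bypassing, and slow effects.
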(event `self.ReceiveBeginPlay`
  (`parent.ReceiveBeginPlay`)
  (bind _returnvalue (`GameplayStatics.GetActorOfClass` "/Game/Merged/Character/AI/BP_AITrack.BP_AITrack_C"))
  (bind _output_get (set `self.Track` _returnvalue))
  (bind _output_get_2 (set `ProjectileMovementComponent.HomingTargetComponent` (`Actor.RootComponent` (`|GetArrayItem` (`/Game/Merged/Character/AI/BP_AITrack.Checkpoints` _output_get))) (`self.ProjectileMovement`)))
  (set `self.Target` _output_get_2))

(event `Update Index`
  (params (Checkpoint :type "/Game/Merged/Track/BP_Checkpoint Object Reference"))
  (bind _checkpoints (`/Game/Merged/Character/AI/BP_AITrack.Checkpoints` (`self.Track`)))
  (bind _output (`|GetArrayItem` _checkpoints (+ (`KismetArrayLibrary.Array_Find` _checkpoints Checkpoint) 1)))
  (bind `_as액터` (cast `Actor` (`KismetMathLibrary.SelectObject` _output (`|GetArrayItem` _checkpoints) (`KismetSystemLibrary.IsValid` _output))))
  (bind _output_get (set `ProjectileMovementComponent.HomingTargetComponent` (`Actor.RootComponent` `_as액터`) (`self.ProjectileMovement`)))
  (set `self.Target` _output_get)
  (`/Engine/EditorBlueprintResources/StandardMacros.IsValid` (`self.Stopover`)
    (:`Is Valid`
      (`self.K2_DestroyActor` (`self.Stopover`))
      (set `self.Bypass` false))))

(event `self.ReceiveTick`
  (params (DeltaSeconds :type "Float (single-precision)"))
  (`self.Set IsDash`)
  (`parent.ReceiveTick` DeltaSeconds)
  (`self.Dash Midway Stop`)
  (`self.Set Speed`)
  (set `self.CharacterVelocity` (`KismetMathLibrary.VSize` (`MovementComponent.Velocity` (`self.ProjectileMovement`))))
  (if (not (`self.Bypass`))
    (bind _forwa (`self.Is Block` 3000.0)
      (:`True`
        (`self.Find Bypass` _forwa 5 100.0)))))

(event `Reset Target`
  (set `ProjectileMovementComponent.HomingTargetComponent` (`self.Target`) (`self.ProjectileMovement`))
  (`KismetSystemLibrary.Delay` 1.0)
  (set `self.Bypass` false))

(fn `UserConstructionScript`)