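; BP_Penguin is the penguin character Blueprint, whose skill input fires a BP_PenguinProj projectile.
; The input passes through a server RPC event to a second RPC event, which checks and sets IsCooldown, plays the Missile sound and spawns the projectile.
; The projectile takes its position and rotation from ProjectileSpawnPos and its scale from ProjSize.
; The cooldown flag is never cleared in this graph, and BeginPlay only calls the parent.
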(event `EnhancedInput|/Game/Merged/Character/Player/Input/Actions/IA_Skill`
  (params (ActionValue :type Boolean) (ElapsedSeconds :type "Float (double-precision)") (TriggeredSeconds :type "Float (double-precision)") (InputAction :type "InputAction Object Reference" :default "/Game/Merged/Character/Player/Input/Actions/IA_Skill.IA_Skill"))
  (:`Started`
    (`self.RPC_Server_SpawnActor_Penguin`)))

(event `RPC_Server_SpawnActor_Penguin`
  (`self.RPC_SpawnActor_Penguin`))

(event `RPC_SpawnActor_Penguin`
  (bind (_returnvalue_location _returnvalue_rotation) (`KismetMathLibrary.BreakTransform` (`SceneComponent.K2_GetComponentToWorld` (`self.Projectile Spawn Pos`))))
  (if (not (`self.IsCooldown`))
    (set `self.IsCooldown` true)
    (`GameplayStatics.PlaySoundAtLocation` "/Game/Assets/SFX/missile.missile" (`self.K2_GetActorLocation`) (struct) 1.0 1.0 0.0 null null null null)
    (`|SpawnActorFromClass` "/Game/Merged/Character/Penguin/BP_PenguinProj.BP_PenguinProj_C" (`KismetMathLibrary.MakeTransform` _returnvalue_location _returnvalue_rotation (`self.ProjSize`)) "Undefined" "MultiplyWithRoot" self null)))

(event `self.ReceiveBeginPlay`
  (`parent.ReceiveBeginPlay`))

(fn `UserConstructionScript`)