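; BP_Penguin_AI is a penguin AI that automatically fires projectiles at objects in front of it.
; Each Tick, after the parent logic, a stationary multi-sphere trace finds nearby objects of the configured types.
; A dot product of each negated hit normal and the forward vector approximates a view cone.
; A passing hit spawns BP_PenguinProj at ProjectileSpawnPos and sets IsCooldown, which this graph never clears.
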(event `self.ReceiveBeginPlay`
  (`parent.ReceiveBeginPlay`))

(event `self.ReceiveTick`
  (params (DeltaSeconds :type "Float (single-precision)"))
  (bind _returnvalue (`self.K2_GetActorLocation`))
  (bind (_returnvalue_location _returnvalue_rotation) (`KismetMathLibrary.BreakTransform` (`SceneComponent.K2_GetComponentToWorld` (`self.Projectile Spawn Pos`))))
  (`parent.ReceiveTick` DeltaSeconds)
  (bind _outhits (`KismetSystemLibrary.SphereTraceMultiForObjects` _returnvalue _returnvalue 2000.0 (`self.Object Types_0`)))
  (for _array_element _outhits
    (if (> (`KismetMathLibrary.Dot_VectorVector` (`KismetMathLibrary.NegateVector` (`.Normal` (`GameplayStatics.BreakHitResult` _array_element))) (`self.GetActorForwardVector`)) 0.6)
      (if (not (`self.IsCooldown`))
        (set `self.IsCooldown` true)
        (`|SpawnActorFromClass` "/Game/Merged/Character/Penguin/BP_PenguinProj.BP_PenguinProj_C" (`KismetMathLibrary.MakeTransform` _returnvalue_location _returnvalue_rotation (`self.ProjSize`)) "Undefined" "MultiplyWithRoot" self null)))))

(fn `UserConstructionScript`)