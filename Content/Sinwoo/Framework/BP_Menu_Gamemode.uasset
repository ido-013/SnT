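; Game mode for the menu that manages players joining the lobby and keeps their profile lists in sync.
; On the lobby map, it records each new player's BP_MenuController, has it create the lobby menu and run setup, then passes it the first connected player's profile as room info.
; UpdateLobby rebuilds the profile list from all connected controllers and pushes it to each one when the player-names flag is set.
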(event `self.HandleStartingNewPlayer`
  (params (NewPlayer :type "PlayerController Object Reference"))
  (bind _all_connectedplayers (`self.All_ConnectedPlayers`))
  (bind _returnvalue (`GameplayStatics.GetCurrentLevelName` true))
  (switch `string` _returnvalue
    (:`LobbyMenu_Map`
      (bind _asbp_menu_controller (cast `/Game/Sinwoo/Framework/BP_MenuController` NewPlayer))
      (`KismetArrayLibrary.Array_Add` _all_connectedplayers _asbp_menu_controller)
      (`/Game/Sinwoo/Framework/BP_MenuController.CreateLobbyMenu` _asbp_menu_controller)
      (`/Game/Sinwoo/Framework/BP_MenuController.Initial_Setup` _asbp_menu_controller)
      (`/Game/Sinwoo/Framework/BP_MenuController.UpdateRoomInfo` _asbp_menu_controller (`/Game/Sinwoo/Framework/BP_MenuController.PlayerProfileInfo` (`|GetArrayItem` _all_connectedplayers))))))

(event `UpdateLobby`
  (params (PlayerNames :type Boolean))
  (if PlayerNames
    (`KismetArrayLibrary.Array_Clear` (`self.All_PlayerProfiles`))
    (for _array_element (`self.All_ConnectedPlayers`)
      (`KismetArrayLibrary.Array_Add` (`self.All_PlayerProfiles`) (`/Game/Sinwoo/Framework/BP_MenuController.PlayerProfileInfo` _array_element)))
    (for _array_element_2 (`self.All_ConnectedPlayers`)
      (if PlayerNames
        (`/Game/Sinwoo/Framework/BP_MenuController.UpdatePlayerNames` _array_element_2 (`self.All_PlayerProfiles`))))))

(fn `UserConstructionScript`)